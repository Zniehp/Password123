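; Simple NPC character that moves toward the first player character on BeginPlay and destroys itself when it takes any damage.
; Helper functions apply damage to the player, test whether the player is farther than a range threshold, check for a playing attack montage, and destroy the NPC.
; Two montage-based attack chains, one destroying the player pawn and one pausing movement during the animation, are disconnected and never run.
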(event `self.ReceiveActorBeginOverlap`
  (params (OtherActor :type "Actor Object Reference")))

(event `self.ReceiveTick`
  (params (DeltaSeconds :type "Float (single-precision)")))

(event `self.ReceiveAnyDamage`
  (params (Damage :type "Float (single-precision)") (DamageType :type "DamageType Object Reference") (InstigatedBy :type "Controller Object Reference") (DamageCauser :type "Actor Object Reference"))
  (`self.K2_DestroyActor`))

(event `self.ReceiveBeginPlay`
  (`|AIMoveTo` self (0.0 0.0 0.0) (`GameplayStatics.GetPlayerCharacter` 0)))

(fn `DAmage`
  (`GameplayStatics.ApplyDamage` (`GameplayStatics.GetPlayerCharacter` 0) (`self.Base Damage`)))

(fn `IS ATTACKING`
  (returns (NewParam :type Boolean))
  (return (`AnimInstance.Montage_IsPlaying` (`SkeletalMeshComponent.GetAnimInstance` (`self.Mesh`)) "/Game/Ai/NPC_anim/Enachnced/Anim_montage_npc.Anim_montage_npc")))

(fn `RANGE`
  (returns (NewParam :type Boolean))
  (return (> (`self.GetDistanceTo` (`GameplayStatics.GetPlayerCharacter` 0)) (`self.Var_Range`))))

(fn `UserConstructionScript`)

(fn `vaaatab`
  (`self.K2_DestroyActor` self))